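; BP_Soda is a consumable soda pickup that the player drinks when nearby.
; On BeginPlay it finds the BP_ThirdPersonCharacter and binds to its EatGarbage event, which calls DrinkSoda and destroys the soda if the player is within range.
; Tick shows the Indicator component only within that same range and spins its yaw by a fixed, frame-rate-dependent step.
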(event `self.ReceiveBeginPlay`
  (bind _outactors (`GameplayStatics.GetAllActorsOfClass` "/Game/ThirdPerson/Blueprints/BP_ThirdPersonCharacter.BP_ThirdPersonCharacter_C"))
  (for _array_element _outactors
    (set `self.Player` _array_element))
  (add `/Game/ThirdPerson/Blueprints/BP_ThirdPersonCharacter.EatGarbage` (`self.Player`) (delegate `CustomEvent`)))

(event `self.ReceiveTick`
  (params (DeltaSeconds :type "Float (single-precision)"))
  (bind _indicator (`self.Indicator`))
  (bind (_relativerotation_roll _relativerotation_pitch _relativerotation_yaw) (`KismetMathLibrary.BreakRotator` (`SceneComponent.RelativeRotation` _indicator)))
  (`SceneComponent.SetHiddenInGame` _indicator (> (`self.GetDistanceTo` (`GameplayStatics.GetPlayerCharacter` 0) self) 500.0) true)
  (`SceneComponent.K2_SetRelativeRotation` _indicator (`KismetMathLibrary.MakeRotator` _relativerotation_roll _relativerotation_pitch (+ _relativerotation_yaw 1.0)) false false))

(event `CustomEvent`
  (if (< (`self.GetDistanceTo` (`GameplayStatics.GetPlayerCharacter` 0) self) 500.0)
    (`/Game/ThirdPerson/Blueprints/BP_ThirdPersonCharacter.DrinkSoda` (`self.Player`))
    (`self.K2_DestroyActor`)))

(fn `UserConstructionScript`)