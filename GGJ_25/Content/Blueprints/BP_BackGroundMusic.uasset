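; BP_BackGroundMusic plays a three-part Bigfoot threat music sequence as non-positional 2D background audio.
; On BeginPlay it spawns one audio component with auto-destroy off, so the same component can be reused for every cue.
; Delays matching each cue's duration chain the switch from threat1 to threat2 to threat3, with no restart logic after the last.
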(event `self.ReceiveBeginPlay`
  (bind _sound (`self.Sound`))
  (bind _sound_2 (`self.Sound`))
  (bind _returnvalue (`GameplayStatics.SpawnSound2D` "/Game/Sound/Bigfoot_mus_threat1_Cue.Bigfoot_mus_threat1_Cue" 1.0 1.0 0.0 null false false))
  (bind _output_get (set `self.Sound` _returnvalue))
  (`KismetSystemLibrary.Delay` (`SoundBase.Duration` (`AudioComponent.Sound` _output_get)))
  (`AudioComponent.SetSound` _sound_2 "/Game/Sound/Bigfoot_mus_threat2_Cue.Bigfoot_mus_threat2_Cue")
  (`AudioComponent.Play` _sound_2 0.0)
  (`KismetSystemLibrary.Delay` (`SoundBase.Duration` (`AudioComponent.Sound` _sound_2)))
  (`AudioComponent.SetSound` _sound "/Game/Sound/Bigfoot_mus_threat3_Cue.Bigfoot_mus_threat3_Cue")
  (`AudioComponent.Play` _sound 0.0))

(fn `UserConstructionScript`)