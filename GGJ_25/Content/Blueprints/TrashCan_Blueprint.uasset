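; Trash can actor that the player can eat for score when nearby.
; On BeginPlay it finds the third-person character and binds to its EatGarbage event dispatcher.
; Tick shows an indicator only while the player is within range.
; When the event fires in range, the can raises the player's score and dirty values, then destroys itself.
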(event `self.ReceiveBeginPlay`
  (bind _outactors (`GameplayStatics.GetAllActorsOfClass` "/Game/ThirdPerson/Blueprints/BP_ThirdPersonCharacter.BP_ThirdPersonCharacter_C"))
  (for _array_element _outactors
    (set `self.Player` _array_element))
  (add `/Game/ThirdPerson/Blueprints/BP_ThirdPersonCharacter.EatGarbage` (`self.Player`) (delegate `CustomEvent`)))

(event `CustomEvent`
  (if (< (`self.GetDistanceTo` (`GameplayStatics.GetPlayerCharacter` 0) self) 500.0)
    (`/Game/ThirdPerson/Blueprints/BP_ThirdPersonCharacter.UpdateScore` (`self.Player`) 100.0)
    (`/Game/ThirdPerson/Blueprints/BP_ThirdPersonCharacter.UpdateDirty` (`self.Player`) 5.0)
    (`self.K2_DestroyActor`)))

(event `self.ReceiveTick`
  (params (DeltaSeconds :type "Float (single-precision)"))
  (`SceneComponent.SetHiddenInGame` (`self.Indicator`) (> (`self.GetDistanceTo` (`GameplayStatics.GetPlayerCharacter` 0) self) 500.0) false))

(fn `UserConstructionScript`)