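; Possessable pawn for the shower cleaning minigame, where the player scrubs BP_ThirdPersonCharacter with a brush.
; Touch drags or IA_Clean move the brush using boundary markers, and a line trace from it lowers or updates the character's dirt, randomly spawning soap and sounds.
; Possession toggles the shower wall and spotlight and ducks background music.
; IA_Interact returns control to the character, restores the scene and clears soap.
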(event `self.ReceiveBeginPlay`
  (set `self.BrushStartPos` (`SceneComponent.K2_GetComponentLocation` (`self.ScrubBrush`)))
  (`SceneComponent.SetVisibility` (`self.Shower Wall2`) true false)
  (`SceneComponent.SetVisibility` (`self.SpotLight1`) false false)
  (`AudioComponent.Stop` (`self.Music`)))

(event `self.ReceivePossessed`
  (params (NewController :type "Controller Object Reference"))
  (`SceneComponent.SetVisibility` (`self.Shower Wall2`) false false)
  (`SceneComponent.SetVisibility` (`self.SpotLight1`) true false)
  (bind _outactors (`GameplayStatics.GetAllActorsOfClass` "/Game/Blueprints/BP_BackGroundMusic.BP_BackGroundMusic_C"))
  (for _array_element _outactors
    (`AudioComponent.AdjustVolume` (`/Game/Blueprints/BP_BackGroundMusic.Sound` _array_element) 1.0 0.1 "Linear")))

(event `UpdateTouchPos`
  (params (EndPos :type "Vector2D Structure"))
  (bind (_returnvalue_x _returnvalue_y) (`KismetMathLibrary.BreakVector2D` (- EndPos (`self.TouchStartPos`))))
  (set `self.CleanX` (* _returnvalue_x -0.5))
  (set `self.CleanY` (* _returnvalue_y -0.5)))

(event `EnhancedInput|/Game/ThirdPerson/Input/Actions/IA_Interact`
  (params (ActionValue :type Boolean) (ElapsedSeconds :type "Float (double-precision)") (TriggeredSeconds :type "Float (double-precision)") (InputAction :type "InputAction Object Reference" :default "/Game/ThirdPerson/Input/Actions/IA_Interact.IA_Interact"))
  (bind _scrubbrush (`self.ScrubBrush`))
  (:`Started`
    (bind _outactors (`GameplayStatics.GetAllActorsOfClass` "/Game/ThirdPerson/Blueprints/BP_ThirdPersonCharacter.BP_ThirdPersonCharacter_C"))
    (for _array_element _outactors
      (`Controller.Possess` (`GameplayStatics.GetPlayerController` 0) _array_element)
      (`SceneComponent.K2_SetWorldLocation` _scrubbrush (`self.BrushStartPos`) false false)
      (`SceneComponent.SetVisibility` _scrubbrush false false)
      (`SceneComponent.SetVisibility` (`self.Shower Wall2`) true false)
      (`SceneComponent.SetVisibility` (`self.SpotLight1`) false false)
      (bind _outactors_2 (`GameplayStatics.GetAllActorsOfClass` "/Game/Blueprints/BP_BackGroundMusic.BP_BackGroundMusic_C"))
      (for _array_element_2 _outactors_2
        (`AudioComponent.AdjustVolume` (`/Game/Blueprints/BP_BackGroundMusic.Sound` _array_element_2) 1.0 1.0 "Linear")
        (`AudioComponent.Stop` (`self.Music`))
        (bind _outactors_3 (`GameplayStatics.GetAllActorsOfClass` "/Game/Characters/BP_Soap.BP_Soap_C"))
        (for _array_element_3 _outactors_3
          (`self.K2_DestroyActor` _array_element_3))))))

(event `InputTouch`
  (params (Location :type "Vector Structure") (FingerIndex :type "ETouchIndex Enum"))
  (bind _scrubbrush (`self.ScrubBrush`))
  (bind _noises (`self.Noises`))
  (bind _scrubbrush_2 (`self.ScrubBrush`))
  (bind (_returnvalue_x _returnvalue_y _returnvalue_z) (`KismetMathLibrary.BreakVector` (`SceneComponent.K2_GetComponentLocation` _scrubbrush_2)))
  (bind (_returnvalue_x_2 _returnvalue_y_2) (`KismetMathLibrary.BreakVector` (`SceneComponent.K2_GetComponentLocation` (`self.LeftBoundPos`))))
  (bind (_returnvalue_x_3 _returnvalue_y_3) (`KismetMathLibrary.BreakVector` (`SceneComponent.K2_GetComponentLocation` (`self.RightBoundPos`))))
  (bind (_returnvalue_x_4 _returnvalue_y_4 _returnvalue_z_2) (`KismetMathLibrary.BreakVector` (`SceneComponent.K2_GetComponentLocation` (`self.TopBoundPos`))))
  (bind (_returnvalue_x_5 _returnvalue_y_5 _returnvalue_z_3) (`KismetMathLibrary.BreakVector` (`SceneComponent.K2_GetComponentLocation` (`self.BottomBoundPos`))))
  (bind (_returnvalue_x_6 _returnvalue_y_6 _returnvalue_z_4) (`KismetMathLibrary.BreakVector` (`SceneComponent.K2_GetComponentLocation` _scrubbrush)))
  (bind _returnvalue (+ _returnvalue_y_6 (`self.CleanX`)))
  (bind _returnvalue_2 (+ _returnvalue_z_4 (`self.CleanY`)))
  (:`Pressed`
    (set `self.TouchStartPos` (`KismetMathLibrary.MakeVector2D` Location_X Location_Y) :!label _label))
  (:`Moved`
    (`self.UpdateTouchPos` (`KismetMathLibrary.MakeVector2D` Location_X Location_Y))
    (`|ExecutionSequence`
      (:`then_0`
        (goto _label))
      (:`then_1`
        (if (>= _returnvalue_y_2 _returnvalue) :!label _label_2
          (set `self.NewY` _returnvalue_y_2)
          (else
            (set `self.NewY` _returnvalue)))
        (if (<= _returnvalue_y_3 _returnvalue)
          (set `self.NewY` _returnvalue)
          (else
            (set `self.NewY` _returnvalue_y_3)))
        (if (>= _returnvalue_z_2 _returnvalue_2)
          (set `self.NewZ` _returnvalue_z_2)
          (else
            (set `self.NewZ` _returnvalue_2)))
        (if (<= _returnvalue_z_3 _returnvalue_2)
          (set `self.NewZ` _returnvalue_2)
          (else
            (set `self.NewZ` _returnvalue_z_3)))
        (`SceneComponent.K2_SetWorldLocation` _scrubbrush (`KismetMathLibrary.MakeVector` _returnvalue_x_6 (`self.NewY`) (`self.NewZ`)) false false)
        (bind _outhit (`KismetSystemLibrary.LineTraceSingle` :`Start` (`SceneComponent.K2_GetComponentLocation` _scrubbrush_2) :`End` (`KismetMathLibrary.MakeVector` (+ _returnvalue_x -100.0) _returnvalue_y _returnvalue_z) :`TraceChannel` "TraceTypeQuery3" :`DrawTime` 10.0))
        (bind _asbp_third_person_character (cast `/Game/ThirdPerson/Blueprints/BP_ThirdPersonCharacter` (`.HitActor` (`GameplayStatics.BreakHitResult` _outhit))))
        (if (> (`KismetMathLibrary.RandomFloat`) 0.5)
          (if (and (not (`AudioComponent.IsPlaying` _noises)) (> (`KismetMathLibrary.RandomFloat`) 0.9))
            (`AudioComponent.Play` _noises 0.0))
          (`|SpawnActorFromClass` "/Game/Characters/BP_Soap.BP_Soap_C" (`KismetMathLibrary.MakeTransform` (`.Location` (`GameplayStatics.BreakHitResult` _outhit))) "Undefined" "MultiplyWithRoot" null null)
          (`AudioComponent.Play` (`self.BubbleSound`) 0.0))
        (if (>= (`/Game/ThirdPerson/Blueprints/BP_ThirdPersonCharacter.DirtyAmount` _asbp_third_person_character) 0.0)
          (`/Game/ThirdPerson/Blueprints/BP_ThirdPersonCharacter.UpdateDirty` _asbp_third_person_character (`self.CleanAmount`)))))))

(event `EnhancedInput|/Game/ThirdPerson/Input/Actions/IA_Clean`
  (params (ActionValue :type "Vector2D Structure") (ElapsedSeconds :type "Float (double-precision)") (TriggeredSeconds :type "Float (double-precision)") (InputAction :type "InputAction Object Reference" :default "/Game/ThirdPerson/Input/Actions/IA_Clean.IA_Clean"))
  (:`Triggered`
    (set `self.CleanX` (* ActionValue_X -10.0))
    (set `self.CleanY` (* ActionValue_Y 10.0))
    (goto _label_2)))

(fn `UserConstructionScript`)