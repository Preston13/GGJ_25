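; BP_EnemyCharacter is an AI-driven enemy character that wanders until it detects the player.
; On BeginPlay it gets its AI controller, runs the BT_Enemy behavior tree and sets a Blackboard enum to the wander state.
; PawnSensing sight and hearing events switch that enum to the chase state when the sensed pawn is a BP_ThirdPersonCharacter.
; Nothing in this Blueprint switches the state back to wander after a chase begins.
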(event `self.ReceiveBeginPlay`
  (bind _output_get (set `self.ControllerRef` (`AIBlueprintHelperLibrary.GetAIController` self)))
  (`AIController.RunBehaviorTree` _output_get "/Game/AI/BT_Enemy.BT_Enemy")
  (`BlackboardComponent.SetValueAsEnum` (`AIBlueprintHelperLibrary.GetBlackboard` (`self.ControllerRef`)) (`self.Key Name`) (`self.WanderState`)))

(event `self.PawnSensing.OnSeePawn`
  (params (Pawn :type "Pawn Object Reference"))
  (bind _asbp_third_person_character (cast `/Game/ThirdPerson/Blueprints/BP_ThirdPersonCharacter` Pawn))
  (`/Engine/EditorBlueprintResources/StandardMacros.IsValid` _asbp_third_person_character
    (:`Is Valid`
      (`BlackboardComponent.SetValueAsEnum` (`AIBlueprintHelperLibrary.GetBlackboard` (`self.ControllerRef`)) (`self.Key Name`) (`self.ChaseState`)))))

(event `self.PawnSensing.OnHearNoise`
  (params (Instigator :type "Pawn Object Reference") (Location :type "Vector Structure (by ref)") (Volume :type "Float (single-precision)"))
  (bind _asbp_third_person_character (cast `/Game/ThirdPerson/Blueprints/BP_ThirdPersonCharacter` Instigator))
  (`/Engine/EditorBlueprintResources/StandardMacros.IsValid` _asbp_third_person_character
    (:`Is Valid`
      (`BlackboardComponent.SetValueAsEnum` (`AIBlueprintHelperLibrary.GetBlackboard` (`self.ControllerRef`)) (`self.Key Name`) (`self.ChaseState`)))))

(fn `UserConstructionScript`)